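; Abducting enemy spaceship that moves in to chase a cow, then flies back, and is destroyed by any damage.
; ChaseToCow and ComeBack set state flags that Tick reads to sweep the ship backward or forward along its forward vector, with chasing taking priority.
; Once it is returning and has not been rendered recently, it calls CowAbducted once on the player controller's UI.
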(event `self.ReceiveTick`
  (params (DeltaSeconds :type "Float (single-precision)"))
  (`self.Abduct`)
  (if (`self.WasRecentlyRendered` 0.8)
    _
    (elif (`self.bIsComingBack`)
      (`/Engine/EditorBlueprintResources/StandardMacros.DoOnce` false
        (:`Completed`
          (`/Game/Blueprints/UI/PlayerUI_W.CowAbducted` (`/Game/Blueprints/CharacterController/PlayerController_BP.Player UI` (`self.PlayerController`))))))))

(event `self.ReceiveBeginPlay`
  (bind _returnvalue (`GameplayStatics.GetActorOfClass` "/Game/Blueprints/CharacterController/PlayerController_BP.PlayerController_BP_C"))
  (set `self.PlayerController` _returnvalue))

(event `self.ReceiveAnyDamage`
  (params (Damage :type "Float (single-precision)") (DamageType :type "DamageType Object Reference") (InstigatedBy :type "Controller Object Reference") (DamageCauser :type "Actor Object Reference"))
  (`self.K2_DestroyActor`))

(fn `Abduct`
  (if (`self.bIsChasing`)
    (`self.K2_AddActorWorldOffset` (* (`self.GetActorForwardVector`) -8.0) true)
    (elif (`self.bIsComingBack`)
      (`self.K2_AddActorWorldOffset` (* (`self.GetActorForwardVector`) 8.0) true))))

(fn `ChaseToCow`
  (params (StartChasing :type Boolean))
  (set `self.bIsChasing` StartChasing))

(fn `ComeBack`
  (set `self.bIsComingBack` true))

(fn `UserConstructionScript`)