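; Cow actor for the abducting enemy that can be lifted and shrunk as if pulled up by a UFO.
; While the abducting flag set by StartAbducting is on, Tick moves it upward and scales it down, hiding its Cylinder component after a short delay.
; UFODestroyed clears the flag, teleports the cow back to its BeginPlay position, restores its scale and shows the Cylinder again.
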(event `self.ReceiveBeginPlay`
  (set `self.StartPosition` (`self.K2_GetActorLocation`)))

(event `self.ReceiveTick`
  (params (DeltaSeconds :type "Float (single-precision)"))
  (if (`self.bIsAbducting`)
    (`self.K2_AddActorWorldOffset` (* (`self.GetActorUpVector`) 4.0))
    (`self.SetActorScale3D` (- (`self.GetActorScale3D`) (* DeltaSeconds 0.5)))
    (`KismetSystemLibrary.Delay` 2.0)
    (`SceneComponent.SetHiddenInGame` (`self.Cylinder`) true true)))

(fn `Start Abducting`
  (params (Activate :type Boolean))
  (set `self.bIsAbducting` Activate))

(fn `UFODestroyed`
  (`|ExecutionSequence`
    (:`then_0`
      (set `self.bIsAbducting` false))
    (:`then_1`
      (`self.K2_SetActorLocation` (`self.StartPosition`) false true)
      (`self.SetActorScale3D` (1.0 1.0 1.0))
      (`SceneComponent.SetHiddenInGame` (`self.Cylinder`) false false))))

(fn `UserConstructionScript`)