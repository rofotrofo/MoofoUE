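; Enemy actor that runs a UFO cow abduction, spawning a spaceship at its Spawner to chase its child-actor cow.
; Tick compares positions to switch the ship between chasing, abducting and returning, using the cow's StartAbducting and the ship's ComeBack.
; A returning ship that passes the Spawner proximity check is destroyed along with this actor.
; If the ship becomes invalid, the cow is notified and a replacement spawns after a delay.
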(event `self.ReceiveBeginPlay`
  (bind _ascow_bp (cast `/Game/Blueprints/Enemies/AbductingEnemy/Cow_BP` (`ChildActorComponent.ChildActor` (`self.Cow_BP`))))
  (set `self.Cow Reference` _ascow_bp)
  (bind _output_get (`self.SpawnNewUFO`))
  (`/Game/Blueprints/Enemies/AbductingEnemy/Spaceship_BP.ChaseToCow` _output_get true))

(event `self.ReceiveTick`
  (params (DeltaSeconds :type "Float (single-precision)"))
  (bind _returnvalue_x (`KismetMathLibrary.BreakVector` (`SceneComponent.K2_GetComponentLocation` (`self.Spawner`))))
  (bind _returnvalue_x_2 (`KismetMathLibrary.BreakVector` (`SceneComponent.K2_GetComponentLocation` (`self.Cow_BP`))))
  (bind (_returnvalue_x_3 _returnvalue_y _returnvalue_z) (`KismetMathLibrary.BreakVector` (`SceneComponent.K2_GetComponentLocation` (`Actor.RootComponent` (`self.Cow Reference`)))))
  (bind _returnvalue_x_4 (`KismetMathLibrary.BreakVector` (`SceneComponent.K2_GetComponentLocation` (`Actor.RootComponent` (`self.Current SpaceShip`)))))
  (bind _returnvalue_x_5 (`KismetMathLibrary.BreakVector` (`SceneComponent.K2_GetComponentLocation` (`Actor.RootComponent` (`self.Current SpaceShip`)))))
  (bind (_returnvalue_x_6 _returnvalue_y_2 _returnvalue_z_2) (`KismetMathLibrary.BreakVector` (`SceneComponent.K2_GetComponentLocation` (`Actor.RootComponent` (`self.Current SpaceShip`)))))
  (if (`KismetSystemLibrary.IsValid` (`self.Current SpaceShip`))
    (if (< (- _returnvalue_x_2 _returnvalue_x_4) 1.0)
      (if (`/Game/Blueprints/Enemies/AbductingEnemy/Spaceship_BP.bIsComingBack` (`self.Current SpaceShip`))
        (if (< (- _returnvalue_x _returnvalue_x_5) 10.0)
          (`self.K2_DestroyActor` (`self.Current SpaceShip`))
          (`self.K2_DestroyActor`)))
      (else
        (`/Game/Blueprints/Enemies/AbductingEnemy/Spaceship_BP.ChaseToCow` (`self.Current SpaceShip`) false)
        (`/Game/Blueprints/Enemies/AbductingEnemy/Cow_BP.Start Abducting` (`self.Cow Reference`) true)
        (if (< (- _returnvalue_z_2 _returnvalue_z) 10.0)
          (`/Game/Blueprints/Enemies/AbductingEnemy/Cow_BP.Start Abducting` (`self.Cow Reference`) false)
          (`/Game/Blueprints/Enemies/AbductingEnemy/Spaceship_BP.ComeBack` (`self.Current SpaceShip`)))))
    (else
      (`/Game/Blueprints/Enemies/AbductingEnemy/Cow_BP.UFODestroyed` (`self.Cow Reference`))
      (`KismetSystemLibrary.Delay` 3.0)
      (bind _output_get (`self.SpawnNewUFO`))
      (bind _output_get_2 (set `self.Current SpaceShip` _output_get))
      (`/Game/Blueprints/Enemies/AbductingEnemy/Spaceship_BP.ChaseToCow` _output_get_2 true))))

(fn `IstheSpaceshipOnTheCow`)

(fn `SpawnNewUFO`
  (returns (Output_Get :type "/Game/Blueprints/Enemies/AbductingEnemy/Spaceship_BP Object Reference"))
  (bind _spawner (`self.Spawner`))
  (bind _returnvalue (`|SpawnActorFromClass` "/Game/Blueprints/Enemies/AbductingEnemy/Spaceship_BP.Spaceship_BP_C" (`KismetMathLibrary.MakeTransform` (`SceneComponent.K2_GetComponentLocation` _spawner) (`SceneComponent.K2_GetComponentRotation` _spawner)) "Undefined" "MultiplyWithRoot" null null))
  (bind _output_get (set `self.Current SpaceShip` _returnvalue))
  (return _output_get))

(fn `UserConstructionScript`)