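; Bonus enemy for the endless mode, a physics cube that awards score when damaged and destroys itself if it falls below a height limit.
; Each hit costs one health and either toggles physics off and on before launching the cube upward for points, or, at depletion, grants a larger reward and destroys it.
; Score is stored on PlayerController_BP and pushed to the UI through Endless_GM.
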(event `self.ReceiveTick`
  (params (DeltaSeconds :type "Float (single-precision)"))
  (bind (_returnvalue_x _returnvalue_y _returnvalue_z) (`KismetMathLibrary.BreakVector` (`SceneComponent.K2_GetComponentLocation` (`self.Cube`))))
  (if (< _returnvalue_z -450.0)
    (`self.K2_DestroyActor`)))

(event `self.ReceiveAnyDamage`
  (params (Damage :type "Float (single-precision)") (DamageType :type "DamageType Object Reference") (InstigatedBy :type "Controller Object Reference") (DamageCauser :type "Actor Object Reference"))
  (bind _health (`self.Health`))
  (set `self.Health` (- _health 1.0))
  (if (< _health 1.0)
    (bind _asplayer_controller_bp (cast `/Game/Blueprints/CharacterController/PlayerController_BP` (`GameplayStatics.GetPlayerController` 0)))
    (bind _output_get (set `/Game/Blueprints/CharacterController/PlayerController_BP.Score` (+ (`/Game/Blueprints/CharacterController/PlayerController_BP.Score` _asplayer_controller_bp) 500) _asplayer_controller_bp))
    (bind _asendless_gm (cast `/Game/Blueprints/GameMode/Endless_GM` (`GameplayStatics.GetGameMode`)))
    (`/Game/Blueprints/UI/PlayerUI_W.RefreshScoreUI` (`/Game/Blueprints/GameMode/Endless_GM.PlayerUI` _asendless_gm) _output_get)
    (`self.K2_DestroyActor`)
    (else
      (`|ExecutionSequence`
        (:`then_0`
          (`self.Deactive physics`))
        (:`then_1`
          (`self.Activate physics`))
        (:`then_2`
          (`PrimitiveComponent.AddImpulse` (`self.Cube`) (0.0 0.0 900.0) "None" true))
        (:`then_3`
          (bind _asplayer_controller_bp_2 (cast `/Game/Blueprints/CharacterController/PlayerController_BP` (`GameplayStatics.GetPlayerController` 0)))
          (bind _output_get_2 (set `/Game/Blueprints/CharacterController/PlayerController_BP.Score` (+ (`/Game/Blueprints/CharacterController/PlayerController_BP.Score` _asplayer_controller_bp_2) 200) _asplayer_controller_bp_2))
          (bind _asendless_gm_2 (cast `/Game/Blueprints/GameMode/Endless_GM` (`GameplayStatics.GetGameMode`)))
          (`/Game/Blueprints/UI/PlayerUI_W.RefreshScoreUI` (`/Game/Blueprints/GameMode/Endless_GM.PlayerUI` _asendless_gm_2) _output_get_2))))))

(fn `Activate physics`
  (bind _cube (`self.Cube`))
  (`|ExecutionSequence`
    (:`then_0`
      (`PrimitiveComponent.SetSimulatePhysics` _cube true))
    (:`then_1`
      (`PrimitiveComponent.SetEnableGravity` _cube true))))

(fn `Deactive physics`
  (bind _cube (`self.Cube`))
  (`|ExecutionSequence`
    (:`then_0`
      (`PrimitiveComponent.SetSimulatePhysics` _cube false))
    (:`then_1`
      (`PrimitiveComponent.SetEnableGravity` _cube false))))

(fn `UserConstructionScript`)