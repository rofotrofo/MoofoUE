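; Player controller for a mouse-aimed shooter that handles firing, ammo, reloading and player lives.
; Shoot traces from the cursor and applies damage: normal rounds hit one actor, while the last round multi-traces as a special bullet and starts a timed reload.
; RecieveDamage removes a life and, when none remain, shows game over and pauses the game.
; UI updates go through the Endless_GM game mode.
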(event `RecieveDamage`
  (bind _asendless_gm (cast `/Game/Blueprints/GameMode/Endless_GM` (`GameplayStatics.GetGameMode`)))
  (`/Game/Blueprints/UI/PlayerUI_W.RecieveDamageUI` (`/Game/Blueprints/GameMode/Endless_GM.PlayerUI` _asendless_gm))
  (bind _output_get (set `self.CurrentLives` (- (`self.CurrentLives`) 1)))
  (if (< _output_get 1)
    (bind _asendless_gm_2 (cast `/Game/Blueprints/GameMode/Endless_GM` (`GameplayStatics.GetGameMode`)))
    (`/Game/Blueprints/GameMode/Endless_GM.Deactivate Player UI` _asendless_gm_2)
    (`/Game/Blueprints/GameMode/Endless_GM.Activate GameOver` _asendless_gm_2)
    (`GameplayStatics.SetGamePaused` true)))

(event `OnReloading`
  (set `self.bIsReloading` true)
  (`KismetSystemLibrary.Delay` (`self.ReloadingTime`))
  (`self.ReloadAmmo`)
  (`/Game/Blueprints/UI/PlayerUI_W.ReloadUI` (`/Game/Blueprints/GameMode/Endless_GM.PlayerUI` (stale `InputAction|Shoot` _asendless_gm))))

(event `InputAction|Shoot`
  (params (Key :type "Key Structure"))
  (bind (_worldlocation _worlddirection) (`self.DeprojectMousePositionToWorld`))
  (bind (_worldlocation_2 _worlddirection_2) (`self.DeprojectMousePositionToWorld`))
  (:`Pressed`
    (if (`self.bIsReloading`)
      _
      (elif (> (`self.CurrentAmmo`) 1)
        (bind _asendless_gm (cast `/Game/Blueprints/GameMode/Endless_GM` (`GameplayStatics.GetGameMode`)))
        (bind _playerui (`/Game/Blueprints/GameMode/Endless_GM.PlayerUI` _asendless_gm))
        (`/Game/Blueprints/UI/PlayerUI_W.ShootUI` _playerui)
        (set `self.CurrentAmmo` (- (`self.CurrentAmmo`) 1))
        ;[1 1 1] Normal bullet
        (bind _outhit (`KismetSystemLibrary.LineTraceSingle` :`Start` _worldlocation_2 :`End` (+ _worldlocation_2 (* _worlddirection_2 (`KismetMathLibrary.Conv_DoubleToVector` 2000.0))) :`TraceChannel` "TraceTypeQuery1" :`DrawDebugType` "ForDuration" :`DrawTime` 4.0))
        (bind (_bblockinghit _binitialoverlap _time _distance _location _impactpoint _normal _impactnormal _physmat _hitactor) (`GameplayStatics.BreakHitResult` _outhit))
        (`KismetSystemLibrary.PrintString` (`KismetSystemLibrary.GetDisplayName` _hitactor))
        (`GameplayStatics.ApplyDamage` _hitactor 1.0)
        (else
          (`self.OnReloading`)
          (cast `/Game/Blueprints/GameMode/Endless_GM` (`GameplayStatics.GetGameMode`))
          (`/Game/Blueprints/UI/PlayerUI_W.ShootUI` _playerui)
          (`/Game/Blueprints/UI/PlayerUI_W.ReloadingModeUI` _playerui)
          ;[1 1 1] Special Bullet
          (bind _outhits (`KismetSystemLibrary.LineTraceMultiForObjects` :`Start` _worldlocation :`End` (+ _worldlocation (* _worlddirection (`KismetMathLibrary.Conv_DoubleToVector` 2000.0))) :`ObjectTypes` (`|MakeArray` "ObjectTypeQuery2" "ObjectTypeQuery4" :!type "EObjectTypeQuery Enum") :`DrawDebugType` "ForDuration" :`TraceColor` (struct :`R` 1.0 :`G` 0.925025 :`A` 1.0) :`DrawTime` 4.0))
          (for _array_element _outhits
            (bind (_bblockinghit_2 _binitialoverlap_2 _time_2 _distance_2 _location_2 _impactpoint_2 _normal_2 _impactnormal_2 _physmat_2 _hitactor_2) (`GameplayStatics.BreakHitResult` _array_element))
            (`KismetSystemLibrary.PrintString` (`KismetSystemLibrary.GetDisplayName` _hitactor_2))
            (`GameplayStatics.ApplyDamage` _hitactor_2 1.0)))))))

(fn `ReloadAmmo`
  (set `self.CurrentAmmo` 4)
  (set `self.bIsReloading` false))

(fn `UserConstructionScript`)