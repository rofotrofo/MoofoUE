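; BasicEnemy_BP is a flying enemy that wanders inside the level's FlightArea_BP volume for a limited lifetime.
; BeginPlay finds the first flight area and, if overlapping it, marks the enemy alive and picks a random point within its bounds.
; Tick eases toward that point with VInterpTo, choosing another on arrival.
; When not alive, it moves toward triple the target vector and self-destructs after a delay; any damage destroys it immediately.
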(event `self.ReceiveTick`
  (params (DeltaSeconds :type "Float (single-precision)"))
  (bind _targetlocation (`self.TargetLocation`))
  (if (`self.bIsAlive`)
    (set `self.ElapsedTime` (+ (`self.ElapsedTime`) DeltaSeconds))
    (bind _output_get (set `self.CurrentLocation` (`self.K2_GetActorLocation`)))
    (`self.K2_SetActorLocation` (`KismetMathLibrary.VInterpTo` _output_get _targetlocation DeltaSeconds 5.0))
    (if (>= (`self.ElapsedTime`) (`self.LifeTime`))
      (set `self.bIsAlive` false)
      (elif (< (`KismetMathLibrary.VSize` (- _targetlocation _output_get)) 5.0)
        (`self.GenerateRandomTarget`)))
    (else
      (set `self.CurrentLocation` (`self.K2_GetActorLocation`))
      (`self.K2_SetActorLocation` (`KismetMathLibrary.VInterpTo` (`self.CurrentLocation`) (* (`self.TargetLocation`) 3) DeltaSeconds 5.0))
      (`KismetSystemLibrary.Delay` 2.0)
      (`self.K2_DestroyActor`))))

(event `self.ReceiveBeginPlay`
  (set `self.ElapsedTime` 0.0)
  (bind _outactors (`GameplayStatics.GetAllActorsOfClass` "/Game/Blueprints/Enemies/FlightArea_BP.FlightArea_BP_C"))
  (bind _output (`|GetArrayItem` _outactors))
  (set `self.Flight Area` (`/Game/Blueprints/Enemies/FlightArea_BP.FlightArea` _output))
  (if (`PrimitiveComponent.IsOverlappingActor` (`self.Collision`) _output)
    (`self.GenerateRandomTarget`)
    (set `self.bIsAlive` true)))

(event `self.ReceiveAnyDamage`
  (params (Damage :type "Float (single-precision)") (DamageType :type "DamageType Object Reference") (InstigatedBy :type "Controller Object Reference") (DamageCauser :type "Actor Object Reference"))
  (`self.K2_DestroyActor`))

(fn `GenerateRandomTarget`
  (bind (_origin _boxextent) (`KismetSystemLibrary.GetComponentBounds` (`self.Flight Area`)))
  (set `self.TargetLocation` (`KismetMathLibrary.MakeVector` (`KismetMathLibrary.RandomFloatInRange` (- (.x _origin) (.x _boxextent)) (+ (.x _origin) (.x _boxextent))) (`KismetMathLibrary.RandomFloatInRange` (- (.y _origin) (.y _boxextent)) (+ (.y _origin) (.y _boxextent))) (`KismetMathLibrary.RandomFloatInRange` (- (.z _origin) (.z _boxextent)) (+ (.z _origin) (.z _boxextent))))))

(fn `UserConstructionScript`)